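; Spawner actor that randomly spawns enemies and fires bullets from its own transform.
; Each Tick makes two independent random rolls, so spawn frequency depends on frame rate: a rare one for an Enemy, a more common one for a scaled-down Bullet.
; Each new Bullet receives the current location of the first PlayerCharacter_BP found in its Stuff variable, presumably as a target.
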(event EventBeginPlay)

(event Collision|EventActorBeginOverlap
  (params (OtherActor :type Actor%20Object%20Reference)))

(event EventTick
  (params (DeltaSeconds :type Float%20%28single-precision%29))
  (bind _returnvalue (Transformation|GetActorTransform))
  (bind (_location _rotation) (Math|Transform|BreakTransform _returnvalue))
  (Utilities|FlowControl|Sequence
    (:then_0
      (if (== (Math|Random|RandomIntegerinRange 0 2000) 13)
        (Game|SpawnActorfromClass "/Script/TGPPair.Enemy" (Transformation|GetActorTransform) "AdjustIfPossibleButDontSpawnIfColliding" 0 0)))
    (:then_1
      (if (== (Math|Random|RandomIntegerinRange 0 130) 13)
        (bind _returnvalue_2 (Game|SpawnActorfromClass "/Game/Blueprints/Bullet.Bullet_C" (Math|Transform|MakeTransform _location _rotation "0.700000,0.700000,0.700000") "AdjustIfPossibleButDontSpawnIfColliding" 0 0))
        (bind _outactors (Actor|GetAllActorsOfClass "/Game/Blueprints/PlayerCharacter_BP.PlayerCharacter_BP_C"))
        (bind _asbullet (Utilities|Casting|CastToBullet _returnvalue_2))
        (Variables|/Game/Blueprints/Bullet.Bullet_C|Setstuff _asbullet (Transformation|GetActorLocation (Utilities|Array|Get(acopy) _outactors)))))))

(fn ConstructionScript)