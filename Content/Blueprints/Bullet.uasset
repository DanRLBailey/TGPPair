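; Bullet projectile actor that steps toward a stored target point (Stuff), damages the player and destroys itself after five seconds.
; Each Tick sphere-traces around itself and calls RemoveHealth on a hit PlayerCharacter_BP, without destroying itself, so damage can repeat.
; Moveto then makes fixed, swept, per-axis steps toward Stuff, independent of delta time.
; The downward Z step also shifts X negatively.
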(event EventBeginPlay
  (Utilities|FlowControl|Delay 5.0)
  (Actor|DestroyActor))

(event Collision|EventActorBeginOverlap
  (params (OtherActor :type Actor%20Object%20Reference)))

(event EventTick
  (params (DeltaSeconds :type Float%20%28single-precision%29))
  (bind _returnvalue (Transformation|GetActorLocation))
  (Utilities|FlowControl|Sequence
    (:then_0
      (bind (_outhit _returnvalue_2) (Collision|SphereTraceForObjects _returnvalue _returnvalue 1e+02 (Utilities|Array|MakeArray "ObjectTypeQuery1" "ObjectTypeQuery1" "ObjectTypeQuery3" "ObjectTypeQuery4" "ObjectTypeQuery5" "ObjectTypeQuery6") false 0 "None"))
      (if _returnvalue_2
        (bind _asplayer_character_bp (Utilities|Casting|CastToPlayerCharacter_BP (.HitActor (Collision|BreakHitResult _outhit))))
        (Default|RemoveHealth _asplayer_character_bp 25)))
    (:then_1
      (CallFunction|Moveto))))

(fn ConstructionScript)

(fn Moveto
  (Utilities|FlowControl|Sequence
    (:then_0
      (if (> (.X (Math|Vector|BreakVector (Variables|Default|Getstuff))) (+ (.X (Math|Vector|BreakVector (Transformation|GetActorLocation))) 1e+01))
        (Transformation|SetActorLocation (+ (Transformation|GetActorLocation) "10.000000, 0, 0") true false)
        (elif (< (.X (Math|Vector|BreakVector (Variables|Default|Getstuff))) (+ (.X (Math|Vector|BreakVector (Transformation|GetActorLocation))) -1e+01))
          (Transformation|SetActorLocation (+ (Transformation|GetActorLocation) "-10.000000, 0, 0") true false))))
    (:then_1
      (if (> (.Y (Math|Vector|BreakVector (Variables|Default|Getstuff))) (+ (.Y (Math|Vector|BreakVector (Transformation|GetActorLocation))) 1e+01))
        (Transformation|SetActorLocation (+ (Transformation|GetActorLocation) "0.000000,10.000000, 0") true false)
        (elif (< (.Y (Math|Vector|BreakVector (Variables|Default|Getstuff))) (+ (.Y (Math|Vector|BreakVector (Transformation|GetActorLocation))) -1e+01))
          (Transformation|SetActorLocation (+ (Transformation|GetActorLocation) "0.000000,-10.000000, 0") true false))))
    (:then_2
      (if (> (.Z (Math|Vector|BreakVector (Variables|Default|Getstuff))) (+ (.Z (Math|Vector|BreakVector (Transformation|GetActorLocation))) 1e+01))
        (Transformation|SetActorLocation (+ (Transformation|GetActorLocation) "0.000000, 0,10.000000") true false)
        (elif (< (.Z (Math|Vector|BreakVector (Variables|Default|Getstuff))) (+ (.Z (Math|Vector|BreakVector (Transformation|GetActorLocation))) -1e+01))
          (Transformation|SetActorLocation (+ (Transformation|GetActorLocation) "-10.000000, 0,-10.000000") true false))))))